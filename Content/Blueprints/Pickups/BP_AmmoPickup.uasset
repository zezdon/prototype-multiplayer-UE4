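; Ammo pickup actor that gives spare ammo to the weapon of a character entering its pickup sphere.
; On the PickupSphereEntered event, only the authority checks that the character has a valid weapon, calls GiveAmmo with AmmoToGive, then destroys the pickup.
; Debug prints show the weapon's spare ammo before and after the pickup.
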(event EventBeginPlay)

(event Collision|EventActorBeginOverlap
  (params (OtherActor :type Actor%20Object%20Reference)))

(event EventTick
  (params (DeltaSeconds :type Float%20%28single-precision%29)))

(event EventPickupSphereEntered
  (params (Character :type BR%20Character%20Object%20Reference))
  (bind _weapon (Variables|/Game/FirstPersonBP/Blueprints/BRCharacter.BRCharacter_C|GetWeapon Character))
  (Networking|SwitchHasAuthority
    (:Authority
      (Utilities|IsValid _weapon
        (:Is%20Valid
          (Development|PrintString (Utilities|String|ToString(Text) (Utilities|Text|FormatText "Our sphere ammo is {spareammo}" (Variables|/Game/Blueprints/Weapons/BP_Weapon.BP_Weapon_C|GetCurrentSpareAmmo _weapon))))
          (Default|GiveAmmo _weapon (Variables|Default|GetAmmoToGive))
          (Development|PrintString (Utilities|String|ToString(Text) (Utilities|Text|FormatText "Our sphere ammo after taking the pickup is {spareammo}" (Variables|/Game/Blueprints/Weapons/BP_Weapon.BP_Weapon_C|GetCurrentSpareAmmo _weapon))))
          (Actor|DestroyActor))))))

(fn ConstructionScript
  (|CallParentFunction))